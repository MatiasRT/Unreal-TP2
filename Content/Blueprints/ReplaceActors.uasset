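; ReplaceActors is a utility Blueprint that swaps placed static mesh actors using a given mesh for a replacement actor class.
; Its BPUtility event scans every StaticMeshActor and compares its mesh to the StaticMesh variable.
; Each match gets an actor of ActorReplacement's class spawned at its transform, then is destroyed.
; BeginPlay, Tick, overlap and the construction script are empty, so all work runs through that one event.
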(event Custom|BP%20Utility
  (bind _outactors (Actor|GetAllActorsOfClass "/Script/Engine.StaticMeshActor"))
  (for _array_element _outactors
    (if (== (Variables|/Script/Engine.StaticMeshComponent|GetStaticMesh (Variables|/Script/Engine.StaticMeshActor|GetStaticMeshComponent _array_element)) (Variables|Default|GetStaticMesh))
      (Game|SpawnActorfromClass (Utilities|GetClass (Variables|Default|GetActorReplacement)) (Transformation|GetActorTransform _array_element) "Undefined" 0 0)
      (Actor|DestroyActor _array_element))))

(event EventBeginPlay)

(event Collision|EventActorBeginOverlap
  (params (OtherActor :type Actor%20Object%20Reference)))

(event EventTick
  (params (DeltaSeconds :type Float%20%28single-precision%29)))

(fn ConstructionScript)