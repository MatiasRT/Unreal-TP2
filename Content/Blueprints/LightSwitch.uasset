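; LightSwitch is an interactable actor Blueprint that lets the player toggle a light with the E key while overlapping it.
; Overlap begin and end enable or disable input from player controller 0 and show or hide the FirstPersonHUD through ToggleHUD.
; Pressing E checks that the HUD is visible, then toggles visibility on the Light reference's root component and its children.
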(event EventBeginPlay)

(event EventTick
  (params (DeltaSeconds :type Float%20%28single-precision%29)))

(event Collision|EventActorBeginOverlap
  (params (OtherActor :type Actor%20Object%20Reference))
  (bind _returnvalue (Game|GetPlayerController 0))
  (Input|EnableInput _returnvalue)
  (Default|ToggleHUD (.AsFirst%20Person%20HUD (Utilities|Casting|CastToFirstPersonHUD (HUD|GetHUD _returnvalue))) true))

(event Collision|EventActorEndOverlap
  (params (OtherActor :type Actor%20Object%20Reference))
  (bind _returnvalue (Game|GetPlayerController 0))
  (Input|DisableInput _returnvalue)
  (Default|ToggleHUD (.AsFirst%20Person%20HUD (Utilities|Casting|CastToFirstPersonHUD (HUD|GetHUD _returnvalue))) false))

(event Input|KeyboardEvents|E
  (params (Key :type Key%20Structure))
  (:Pressed
    (bind _hudvisibility (Default|IsHUDVisible (.AsFirst%20Person%20HUD (Utilities|Casting|CastToFirstPersonHUD (HUD|GetHUD (Game|GetPlayerController 0))))))
    (if _hudvisibility
      (Rendering|ToggleVisibility (Variables|/Script/Engine.Actor|GetRootComponent (Variables|Default|GetLight)) true))))

(fn ConstructionScript)